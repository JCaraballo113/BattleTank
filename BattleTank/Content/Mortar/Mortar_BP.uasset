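; Mortar Blueprint that sets up an aimable emplacement with a dome, barrel and floating health bar.
; On BeginPlay it initializes the TankAiming component with the dome as turret and the barrel as barrel.
; It then casts its Widget component's user widget to HealthBar and passes itself as the tank reference.
; Tick, overlap and construction logic are empty.
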(event `self.ReceiveBeginPlay`
  (`TankAimingComponent.Initialize` (`self.TankAiming`) (`self.Mortar Dome`) (`self.Mortar Barrel`))
  (`self.Initialize Health Bar Widget`))

(fn `Initialize Health Bar Widget`
  (bind _ashealth_bar (cast `/Game/UI/HealthBar` (`WidgetComponent.GetUserWidgetObject` (`self.Widget`))))
  (set `/Game/UI/HealthBar.TankRef` self _ashealth_bar))

(fn `UserConstructionScript`)